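; Enemy spawner that places the mobs of the first stage of the "FirstLevel" data table row as BP_BasicEnemy actors.
; The construction script loads the mob list, and BeginPlay caches the player's location and spawns one enemy per entry.
; Enemies form a staggered line offset from the player, receiving health, score and a random box point as spawn offset.
; An older grid-spawn loop remains disconnected.
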(event Custom|SpawnEnemy
  (for (_array_element _array_index) (Variables|Default|GetLevelMob)
    (Game|SpawnActorfromClass "/Game/_Core/Enemy/BP_BasicEnemy.BP_BasicEnemy_C" (Math|Transform|MakeTransform (+ (Variables|Default|GetPlayerloc) "1000.000000,-650.000000, 0" (* "0,350.000000, 0" _array_index) (* "-150.000000,0.000000, 0" (Math|Integer|%(Integer) _array_index 3))) "0,180.000000, 0" "1,1,1") "Undefined" 0 (.Health (Utilities|Struct|BreakMobs _array_element)) (.ScoreAmount (Utilities|Struct|BreakMobs _array_element)) (Math|Random|RandomPointinBoundingBox (Transformation|GetWorldLocation (Variables|Default|GetDefaultSceneRoot)) (Components|Box|GetScaledBoxExtent (Variables|Default|GetBox))) 0)))

(event EventBeginPlay
  (Utilities|FlowControl|Sequence
    (:then_0
      (Variables|Default|SetPlayerRef (.AsBP%20Player (Utilities|Casting|CastToBP_Player (Game|Player|GetPlayerPawn 0))))
      (Variables|Default|SetPlayerloc (Transformation|GetActorLocation (Variables|Default|GetPlayerRef))))
    (:then_1
      (CallFunction|SpawnEnemy))))

(event Collision|EventActorBeginOverlap
  (params (OtherActor :type Actor%20Object%20Reference)))

(event EventTick
  (params (DeltaSeconds :type Float%20%28single-precision%29)))

(fn ConstructionScript
  (bind _returnvalue (Utilities|GetDataTableRow (Variables|Default|GetLevelData) "FirstLevel")
    (:then
      (Variables|Default|SetLevelMob (Utilities|Struct|BreakStageStruct (Utilities|Array|Get(acopy) (.Stages (Utilities|Struct|BreakLevelStruct _returnvalue))))))))