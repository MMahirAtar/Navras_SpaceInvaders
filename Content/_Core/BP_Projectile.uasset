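; BP_Projectile is a projectile actor that damages what it hits and then destroys itself.
; The construction script sets the ProjectileMovement velocity to its owner's forward vector.
; The first hit on Sphere1 applies DamageAmount through the hit actor's BPC_Health component, if present.
; Actors of the same class as the owner take no damage, though the projectile is still destroyed on contact.
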(event OnComponentHit(Sphere1)
  (params (HitComponent :type Primitive%20Component%20Object%20Reference) (OtherActor :type Actor%20Object%20Reference) (OtherComp :type Primitive%20Component%20Object%20Reference) (NormalImpulse :type Vector :default "0, 0, 0") (Hit :type Hit%20Result%20Structure%20%28by%20ref%29))
  (bind _returnvalue (Actor|GetComponentbyClass OtherActor "/Game/_Core/Components/BPC_Health.BPC_Health_C"))
  (Utilities|FlowControl|DoOnce false
    (:Completed
      (if (!= (Utilities|GetClass (Components|GetOwner)) (Utilities|GetClass OtherActor))
        (Utilities|IsValid _returnvalue
          (:Is%20Valid
            (Default|GainDamage _returnvalue (Variables|Default|GetDamage%20Amount)))
          (:Is%20Not%20Valid
            _))
        (Actor|DestroyActor self)
        (else
          (Actor|DestroyActor self))))))

(fn ConstructionScript
  (Variables|/Script/Engine.MovementComponent|SetVelocity (Variables|Default|GetProjectileMovement) (Transformation|GetActorForwardVector (Components|GetOwner))))