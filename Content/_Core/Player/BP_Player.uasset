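; BP_Player is the player's ship, which moves on a horizontal plane and fires projectiles.
; Forward and right axes offset the ship mesh, sideways input also tilts Mesh, and Tick sets the actor location from the ship mesh's position with vector-size clamps on X and Y.
; BPCWeapon is set to BP_Projectile and starts rapid fire on BeginPlay.
; BPCHealth takes the player's max health, and its death event only prints a message.
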(event Custom|Playerdied
  (Development|PrintString "PlayerDied"))

(event EventTick
  (params (DeltaSeconds :type Float%20%28single-precision%29))
  (bind _playershipmesh (Variables|Default|GetPlayerShipMesh))
  (bind _returnvalue (Transformation|GetWorldLocation _playershipmesh))
  (bind (_x _y _z) (Math|Vector|BreakVector _returnvalue))
  (Transformation|SetActorLocation (Math|Vector|MakeVector (.X (Math|Vector|BreakVector (Math|Vector|ClampVectorSize (Math|Vector|MakeVector _x 0.0 0.0) 1e+01 6e+02))) (.Y (Math|Vector|BreakVector (Math|Vector|ClampVectorSize (Math|Vector|MakeVector 0.0 _y 0.0) -1e+03 1e+03))) _z) false false))

(event EventBeginPlay
  (Utilities|FlowControl|Sequence
    (:then_0
      (Default|Rapidfire (Variables|Default|GetBPC_Weapon) 0.5))
    (:then_1
      (Variables|/Game/_Core/Components/BPC_Health.BPC_Health_C|SetMaxHealth (Variables|Default|GetBPC_Health) (Variables|Default|GetPlayerMaxHealth))
      (EventDispatchers|BindEventtoDieEvent (Variables|Default|GetBPC_Health) (delegate Custom|Playerdied)))))

(event Input|AxisEvents|InputAxisMoveForward
  (params (AxisValue :type Float%20%28single-precision%29))
  (Transformation|AddLocalOffset (Variables|Default|GetPlayerShipMesh) (Math|Vector|MakeVector (* AxisValue 2.5) 0.0 0.0) false false))

(event Input|AxisEvents|InputAxisMoveRight
  (params (AxisValue :type Float%20%28single-precision%29))
  (Transformation|AddLocalOffset (Variables|Default|GetPlayerShipMesh) (Math|Vector|MakeVector 0.0 (* AxisValue 2.5) 0.0) false false)
  (Components|MoveComponentTo (Variables|Default|Getmesh) "0, 0, 0" (Math|Rotator|Lerp(Rotator) "0.000000,90.000000, 0" "-30.000000,90.000000,0.000000" AxisValue) false false 0.2 true))

(fn ConstructionScript
  (Variables|/Game/_Core/Components/BPC_Weapon.BPC_Weapon_C|SetProjectileClass (Variables|Default|GetBPC_Weapon) "/Game/_Core/BP_Projectile.BP_Projectile_C"))