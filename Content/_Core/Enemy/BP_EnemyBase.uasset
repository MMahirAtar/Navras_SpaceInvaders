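; Base enemy actor that glides in from an offset to its spawn point while rapid-firing enemy projectiles.
; BeginPlay sets health, binds damage and death events and starts the weapon, while Tick interpolates location at randomized speed.
; Damage triggers effects; death also awards score, notifies the owning spawner and destroys the actor.
; Construction Script sets the projectile class and damage only on an already-placed projectile; level movement events are empty stubs.
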(event Custom|Level%20Enter)

(event Custom|Take%20Position)

(event Custom|Level%20Exit)

(event Custom|OnDied
  (Utilities|FlowControl|Sequence
    (:then_0
      (Effects|SpawnEmitteratLocation (Variables|Default|GetDieParticle) (Transformation|GetActorLocation))
      (Audio|PlaySound2D (Variables|Default|GetDieAudio) 1.0 1.0 0.0 0 0)
      (Default|ScoreUp (Variables|Default|GetBPC_Score) (Variables|Default|GetScoreAmount)))
    (:then_1
      (bind _asbp_enemy_spwaner (Utilities|Casting|CastToBP_EnemySpwaner (Components|GetOwner)))
      (Default|RemoveMob _asbp_enemy_spwaner))
    (:then_2
      (Actor|DestroyActor))))

(event Custom|initEnemy
  (Variables|/Game/_Core/Components/BPC_Health.BPC_Health_C|SetMaxHealth (Variables|Default|GetBPC_Health) (Variables|Default|GetHealth))
  (Default|InitMaxHealth (Variables|Default|GetBPC_Health))
  (CallFunction|EnemyBindings))

(event Custom|EnemyBindings
  (EventDispatchers|BindEventtoGainDamageEvent (Variables|Default|GetBPC_Health) (delegate Custom|GainDamageEvent))
  (EventDispatchers|BindEventtoDieEvent (Variables|Default|GetBPC_Health) (delegate Custom|OnDied))
  (Variables|Default|SetSpawnloc (Transformation|GetActorLocation))
  (Transformation|SetActorLocation (+ (Variables|Default|GetSpawnloc) (Variables|Default|GetSpawnofset)) false false)
  (Default|Rapidfire (Variables|Default|GetBPC_Weapon) (Variables|Default|GetRapidFireTimer)))

(event Custom|GainDamageEvent
  (Audio|PlaySound2D (Variables|Default|GetGainDamageAudio) 1.0 1.0 0.0 0 0)
  (Effects|SpawnEmitteratLocation (Variables|Default|GetDamageParticle) (Transformation|GetActorLocation)))

(event EventBeginPlay
  (CallFunction|InitEnemy))

(event EventTick
  (params (DeltaSeconds :type Float%20%28single-precision%29))
  (Transformation|SetActorLocation (Math|Interpolation|VInterpTo (Transformation|GetActorLocation) (Variables|Default|GetSpawnloc) DeltaSeconds (Math|Random|RandomFloatinRange 0.8 1.2)) false false))

(fn ConstructionScript
  (bind _output_get (Variables|/Game/_Core/Components/BPC_Weapon.BPC_Weapon_C|SetProjectileClass (Variables|Default|GetBPC_Weapon) "/Game/_Core/BP_EnemyProjectile.BP_EnemyProjectile_C"))
  (bind _returnvalue (Actor|GetActorOfClass _output_get))
  (bind _asbp_enemy_projectile (Utilities|Casting|CastToBP_EnemyProjectile _returnvalue))
  (Variables|/Game/_Core/BP_EnemyProjectile.BP_EnemyProjectile_C|SetDamage%20Amount _asbp_enemy_projectile (Variables|Default|GetDamage%20Amount))
  (Development|PrintString (Utilities|String|ToString(Integer) (Variables|/Game/_Core/BP_EnemyProjectile.BP_EnemyProjectile_C|GetDamage%20Amount _asbp_enemy_projectile))))