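; BPC_Health is a health component that tracks current health against a maximum and signals death.
; On BeginPlay it sets current health to MaxHealth.
; GainDamage stores the damage amount minus current health, an operand order reversed from usual damage subtraction, clamped between zero and MaxHealth.
; When the result reaches zero, it calls CallDieEvent.
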(event Custom|Init%20Max%20Health
  (Variables|Default|SetCurrentHealth (Variables|Default|GetMaxHealth)))

(event Custom|GainDamage
  (params (DamageAmount :type Integer))
  (Variables|Default|SetCurrentHealth (Math|Integer|Clamp(Integer) (- DamageAmount (Variables|Default|GetCurrentHealth)) 0 (Variables|Default|GetMaxHealth)))
  (if (<= (Variables|Default|GetCurrentHealth) 0)
    (Default|CallDieEvent)))

(event EventBeginPlay
  (CallFunction|InitMaxHealth))