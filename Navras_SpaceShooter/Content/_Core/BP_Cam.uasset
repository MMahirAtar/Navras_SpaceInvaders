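; BP_Cam is a fixed overhead camera actor that becomes the player's view at game start.
; On BeginPlay it takes the view target, moves above and slightly behind the player pawn, and rotates toward a point ahead of it.
; The placement happens once; Tick is empty, so the camera does not follow the pawn afterward.
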(event EventBeginPlay
  (Game|Player|SetViewTargetwithBlend (Game|GetPlayerController 0) self 0.0 "VTBlend_Linear" 0.0 false)
  (Transformation|SetActorLocation (+ (Transformation|GetActorLocation (Game|Player|GetPlayerPawn 0)) "-300.000000, 0,1500.000000") false false)
  (Transformation|SetActorRotation (Math|Rotator|FindLookatRotation (Transformation|GetActorLocation) (+ (Transformation|GetActorLocation (Game|Player|GetPlayerPawn 0)) "600.000000, 0, 0"))))

(event EventTick
  (params (DeltaSeconds :type Float%20%28single-precision%29)))

(fn ConstructionScript)