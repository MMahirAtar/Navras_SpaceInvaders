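; Spawner actor that populates the level with a grid of BP_EnemyBase enemies once, when play begins.
; SpawnEnemy uses nested loops to fill SpawnLocs with evenly spaced X/Y points from a hardcoded world-space origin, independent of the spawner's own transform.
; It then spawns one enemy at each stored location.
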(event Custom|SpawnEnemy
  (for _index (range 0 5)
    (for _index_2 (range 0 5)
      (Utilities|Array|Add (Variables|Default|GetSpawnLocs) (+ (* "200.000000,0.000000, 0" _index) "500.000000,-600.000000,112.000000" (* "0.000000,200.000000, 0" _index_2)))))
  (for _array_element (Variables|Default|GetSpawnLocs)
    (Game|SpawnActorfromClass "/Game/_Core/BP_EnemyBase.BP_EnemyBase_C" (Math|Transform|MakeTransform _array_element "0, 0, 0" "1,1,1") "Undefined" 0 0)))

(event EventBeginPlay
  (CallFunction|SpawnEnemy))

(event Collision|EventActorBeginOverlap
  (params (OtherActor :type Actor%20Object%20Reference)))

(event EventTick
  (params (DeltaSeconds :type Float%20%28single-precision%29)))

(fn ConstructionScript)